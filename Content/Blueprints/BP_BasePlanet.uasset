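; BP_BasePlanet is a planet actor that hosts a pawn moving across its spherical surface.
; On BeginPlay it spawns a BP_SpherePawn, assigns itself as that pawn's planet and places it at the 2D surface origin.
; It then orders the pawn's spherical movement to a fixed coordinate 360 units along the first axis.
; GetRadius exposes the scaled radius of its Sphere component.
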(event EventBeginPlay
  (bind _returnvalue (Game|SpawnActorfromClass "/Game/Blueprints/BP_SpherePawn.BP_SpherePawn_C" (Math|Transform|MakeTransform "1000.000000,1000.000000,1000.000000") "AdjustIfPossibleButAlwaysSpawn" 0 0))
  (Class|SpherePawn|SetPlanet _returnvalue self)
  (Class|SpherePawn|SetLocationonPlanet _returnvalue)
  (bind _returnvalue_2 (Class|SpherePawn|GetSphericalMovement _returnvalue))
  (Class|SphericalMovement|Moveto _returnvalue_2 "(X=360.000000,Y=0.000000)"))

(fn ConstructionScript)

(fn GetRadius
  (return (Components|Sphere|GetScaledSphereRadius (Variables|Default|GetSphere))))