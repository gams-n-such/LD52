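; Player controller that orbits and zooms the camera around a possessed BP_BasePlanetPawn.
; On possession it caches the pawn, then while left click is held, mouse axes add yaw and pitch input and reset control rotation with zero roll.
; Zoom in and out actions step the pawn's spring arm length by a fixed delta, only when the result stays within the min and max limits.
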(event EventPossess
  (params (PossessedPawn :type Pawn%20Object%20Reference))
  (bind _asbp_base_planet_pawn (Utilities|Casting|CastToBP_BasePlanetPawn PossessedPawn))
  (Variables|Default|SetAs%20BP%20Base%20Planet%20Pawn _asbp_base_planet_pawn))

(event Input|ActionEvents|InputActionZoomIn
  (params (Key :type Key%20Structure :default "None"))
  (bind _as_bp_base_planet_pawn (Variables|Default|GetAs%20BP%20Base%20Planet%20Pawn))
  (bind _springarm (Variables|/Game/Blueprints/BP_BasePlanetPawn.BP_BasePlanetPawn_C|GetSpringArm _as_bp_base_planet_pawn))
  (:Pressed
    (if (not (<= (- (Variables|/Script/Engine.SpringArmComponent|GetTargetArmLength _springarm) (Variables|Input|Zoom|GetDeltaZoom)) (Variables|Input|Zoom|GetMinZoom)))
      (Variables|/Script/Engine.SpringArmComponent|SetTargetArmLength _springarm (- (Variables|/Script/Engine.SpringArmComponent|GetTargetArmLength _springarm) (Variables|Input|Zoom|GetDeltaZoom))))))

(event Input|ActionEvents|InputActionZoomOut
  (params (Key :type Key%20Structure :default "None"))
  (bind _as_bp_base_planet_pawn (Variables|Default|GetAs%20BP%20Base%20Planet%20Pawn))
  (bind _springarm (Variables|/Game/Blueprints/BP_BasePlanetPawn.BP_BasePlanetPawn_C|GetSpringArm _as_bp_base_planet_pawn))
  (:Pressed
    (if (not (>= (+ (Variables|/Script/Engine.SpringArmComponent|GetTargetArmLength _springarm) (Variables|Input|Zoom|GetDeltaZoom)) (Variables|Input|Zoom|GetMaxZoom)))
      (Variables|/Script/Engine.SpringArmComponent|SetTargetArmLength _springarm (+ (Variables|/Script/Engine.SpringArmComponent|GetTargetArmLength _springarm) (Variables|Input|Zoom|GetDeltaZoom))))))

(event Input|ActionEvents|InputActionLeftClick
  (params (Key :type Key%20Structure :default "None"))
  (:Pressed
    (Variables|Input|SetLeftClick true))
  (:Released
    (Variables|Input|SetLeftClick false)))

(event Input|AxisEvents|InputAxisMouseX
  (params (AxisValue :type Float%20%28single-precision%29))
  (bind _as_bp_base_planet_pawn (Variables|Default|GetAs%20BP%20Base%20Planet%20Pawn))
  (bind _returnvalue (Pawn|GetControlRotation _as_bp_base_planet_pawn :!class /Script/Engine.Pawn))
  (if (Variables|Input|GetLeftClick)
    (Pawn|Input|AddControllerYawInput (Variables|Default|GetAs%20BP%20Base%20Planet%20Pawn) AxisValue)
    (Pawn|SetControlRotation (Math|Rotator|MakeRotator 0.0 (.pitch _returnvalue) (.yaw _returnvalue)))))

(event Input|AxisEvents|InputAxisMouseY
  (params (AxisValue :type Float%20%28single-precision%29))
  (bind _as_bp_base_planet_pawn (Variables|Default|GetAs%20BP%20Base%20Planet%20Pawn))
  (bind _returnvalue (Pawn|GetControlRotation _as_bp_base_planet_pawn :!class /Script/Engine.Pawn))
  (if (Variables|Input|GetLeftClick)
    (Pawn|Input|AddControllerPitchInput (Variables|Default|GetAs%20BP%20Base%20Planet%20Pawn) AxisValue)
    (Pawn|SetControlRotation (Math|Rotator|MakeRotator 0.0 (.pitch _returnvalue) (.yaw _returnvalue)))))

(fn ConstructionScript)