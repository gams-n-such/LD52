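; BP_PlayerState holds the player's power, biomass, skill list and captured-city count, broadcasting changes through dispatcher calls.
; CastTheSpell checks and deducts the skill's biomass cost, read from class defaults, then spawns the skill actor and signals success.
; Spawned skills align their Z axis to the planet surface normal, found by a line trace from the spawn point with End left at default.
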(event Custom|SpawnTheSkill
  (params (Skill :type BP%20Base%20Skill%20Class%20Reference) (SpawnLocation :type Vector))
  (Game|SpawnActorfromClass Skill (Math|Transform|MakeTransform SpawnLocation (CallFunction|FindRotatioinfromPlanetNormal SpawnLocation) "1,1,1") "AlwaysSpawn" 0 0))

(event Custom|ChangeCurrentPower
  (params (Damage :type Float%20%28single-precision%29))
  (bind _output_get (Variables|Default|SetCurrentPower (- (Variables|Default|GetCurrentPower) Damage)))
  (Default|CallOnChangeCurrentPower _output_get))

(event Custom|AddSkill
  (params (Skill :type BP%20Base%20Skill%20Class%20Reference))
  (bind _currentskills (Variables|Default|GetCurrentSkills))
  (Utilities|Array|Add _currentskills Skill)
  (Default|CallOnSkillsChangedDispatcher _currentskills))

(event Custom|CityWasCaptured
  (bind _output_get (Variables|Default|SetCurrentCapturedСities (+ (Variables|Default|GetCurrentCapturedСities) 1)))
  (Default|CallOnChangeCapturedCitiesCount _output_get))

(fn ConstructionScript)

(fn IsEnoughtBiomass
  (params (Cost :type Float%20%28single-precision%29))
  (return (>= (Variables|Default|GetCurrentBiomass) Cost)))

(fn CasttheSpell
  (params (Skill :type BP%20Base%20Skill%20Class%20Reference) (SpawnLocation :type Vector))
  (bind _success (CallFunction|SpentbyBiomass Skill))
  (if _success
    (CallFunction|SpawntheSkill Skill SpawnLocation)
    (Default|CallOnSkillCastSuccessed)
    (return true)
    (else
      (return false))))

(fn SpentbyBiomass
  (params (Cost :type BP%20Base%20Skill%20Class%20Reference))
  (bind _skilldata (Utilities|GetClassDefaults Cost))
  (bind _cost (Utilities|Struct|BreakS_SkillData _skilldata))
  (if (CallFunction|IsEnoughtBiomass _cost)
    (bind _output_get (Variables|Default|SetCurrentBiomass (- (Variables|Default|GetCurrentBiomass) _cost)))
    (Default|CallOnChangeCurrentBiomass _output_get)
    (return true)
    (else
      (return false))))

(fn FindRotatioinfromPlanetNormal
  (params (SpawnLocation :type Vector))
  (bind (_outhit _returnvalue) (Collision|LineTraceByChannel SpawnLocation "0, 0, 0" "TraceTypeQuery3" false 0 "None" true "(R=1.000000,G=0.000000,B=0.000000,A=1.000000)" "(R=0.000000,G=1.000000,B=0.000000,A=1.000000)" 2.0))
  (if _returnvalue
    (return (Math|Rotator|MakeRotfromZ (.ImpactNormal (Collision|BreakHitResult _outhit))))
    (else
      (Development|PrintString "Rotation failed. Cant find the Planet Collision. ")
      (return "0, 0, 0"))))