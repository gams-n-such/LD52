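; BP_SpherePawn is a pawn that moves on a spherical planet through its SphericalMovement component.
; BeginPlay runs the parent logic, then passes the pawn's Speed to that component.
; SnapToThePlanet line traces from the pawn toward the default world origin, then teleports it to the hit point with up aligned to the surface normal.
; Nothing in this graph calls the snap function, and Tick is unused.
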(event EventBeginPlay
  (|CallParentFunction)
  (Class|SphericalMovement|SetSpeed (Variables|Default|GetSphericalMovement) (Variables|Default|GetSpeed)))

(event Collision|EventActorBeginOverlap
  (params (OtherActor :type Actor%20Object%20Reference)))

(event EventTick
  (params (DeltaSeconds :type Float%20%28single-precision%29)))

(fn ConstructionScript)

(fn SnaptothePlanet
  (bind (_outhit _returnvalue) (Collision|LineTraceByChannel (Transformation|GetActorLocation) "0, 0, 0" "TraceTypeQuery3" false 0 "ForOneFrame" true "(R=1.000000,G=0.000000,B=0.000000,A=1.000000)" "(R=0.000000,G=1.000000,B=0.000000,A=1.000000)" 2.0))
  (if _returnvalue
    (Transformation|SetActorLocationAndRotation (.ImpactPoint (Collision|BreakHitResult _outhit)) (Math|Rotator|MakeRotfromZ (.ImpactNormal (Collision|BreakHitResult _outhit))) false true)))