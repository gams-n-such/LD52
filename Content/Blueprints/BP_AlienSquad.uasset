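; Alien squad actor that attacks the nearest town and adds its forces to it.
; AttackClosestTown finds the closest town meeting a minimum level, notifies it that it is targeted by enemies, then moves the squad to its location.
; When its sphere begins overlapping a BP_BaseTown, it adds the squad's unit power to that town's alien forces.
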(event OnComponentBeginOverlap(Sphere)
  (params (OverlappedComponent :type Primitive%20Component%20Object%20Reference) (OtherActor :type Actor%20Object%20Reference) (OtherComp :type Primitive%20Component%20Object%20Reference) (OtherBodyIndex :type Integer) (bFromSweep :type Boolean) (SweepResult :type Hit%20Result%20Structure%20%28by%20ref%29))
  (bind _asbp_base_town (Utilities|Casting|CastToBP_BaseTown OtherActor))
  (Default|AddAlienForces _asbp_base_town (.unitpower (Variables|Default|GetSquatData))))

(event EventAttackClosestTown
  (bind _town (CallFunction|GetTownClosesttoPoint (Transformation|GetActorLocation) "NewEnumerator0"))
  (Utilities|IsValid _town
    (:Is%20Valid
      (Utilities|FlowControl|Sequence
        (:then_0
          (Default|HandleTargetedbyEnemies _town 0.0))
        (:then_1
          (Class|SphericalCoordinateSystemBFL|To2D (Transformation|GetActorLocation _town))
          (Class|SpherePawn|Moveto3D (Transformation|GetActorLocation _town)))))))

(fn ConstructionScript
  (|CallParentFunction))