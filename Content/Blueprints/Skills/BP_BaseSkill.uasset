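; BP_BaseSkill is a base skill actor that drops a spore, then spawns troops where the actor stands.
; On BeginPlay it computes a per-frame Z step from the spore's relative height, timeline length and current delta time.
; LandingAnimationTimeline applies that fixed step as a local offset each update, so the descent depends on frame rate.
; When the timeline finishes, it spawns TroopsClass if valid and destroys itself.
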(event Custom|SpawnTroops
  (bind _troopsclass (Variables|Default|GetTroopsClass)
    (:then
      (Game|SpawnActorfromClass _troopsclass (Transformation|GetActorTransform) "AlwaysSpawn" 0 0)
      (Actor|DestroyActor))
    (:else)))

(event EventBeginPlay
  (bind _offsetfromframe (CallFunction|CalculateStepPerFrame))
  (Timeline|LandingAnimationTimeline PlayFromStart
    (:Update
      (Transformation|AddLocalOffset (Variables|Default|GetSpore) (Math|Vector|MakeVector 0.0 0.0 _offsetfromframe) false false))
    (:Finished
      (CallFunction|SpawnTroops))))

(fn ConstructionScript)

(fn CalculateStepPerFrame
  (return (* (/ (.z (Variables|/Script/Engine.SceneComponent|GetRelativeLocation (Variables|Default|GetSpore))) (/ (Components|Timeline|GetTimelineLength (Variables|Default|GetLandingAnimationTimeline)) (Utilities|Time|GetWorldDeltaSeconds))) -1.0)))