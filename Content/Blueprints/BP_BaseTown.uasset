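; Base town actor on the planet, where alien and defender forces fight until the town is captured, rewarding the player with biomass.
; Tick drains both powers during combat, captures at zero defenders, and turns the biomass and power widgets toward the camera.
; Dispatchers broadcast power changes, targeting and capture, while help requests pass eligibility and size checks before spawning reinforcements.
; Construction snaps it to the planet and picks its mesh by type and capture state.
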(event Custom|UpdateMesh
  (bind _result (Combat|IsTownCaptured))
  (bind _meshbytype (Variables|Default|GetMeshByType))
  (bind _type (Variables|Default|GetType))
  (bind _capturedmeshbytype (Variables|Default|GetCapturedMeshByType))
  (bind _returnvalue (select _result _capturedmeshbytype _meshbytype))
  (bind (_value _returnvalue_2) (Utilities|Map|Find _returnvalue _type))
  (if _returnvalue_2
    (Components|StaticMesh|SetStaticMesh (Variables|Default|GetMesh) _value)
    (else
      (Development|PrintString "BP_BaseTown: mesh for town type not found"))))

(event Custom|CaptureTown
  (if (not (Combat|IsTownCaptured))
    (Variables|Combat|SetbIsCaptured true)
    (CallFunction|OnTownCaptured)
    (Default|CallOnTownCapturedDispatcher self)))

(event Custom|OnTownCaptured
  (Utilities|FlowControl|Sequence
    (:then_0
      (CallFunction|UpdateMesh))
    (:then_1
      (bind _asbp_player_state (Utilities|Casting|CastToBP_PlayerState (Variables|/Script/Engine.Controller|GetPlayerState (Game|GetPlayerController 0))))
      (Default|AddBiomass _asbp_player_state (Variables|Default|GetReward))
      (Default|CityWasCaptured _asbp_player_state))))

(event Custom|AddDefenderPower
  (params (NewForces :type Float%20%28single-precision%29))
  (Math|Float|CompareFloat NewForces 0.0
    (:>
      (bind _output_get (Variables|Combat|SetDefenderPower (+ NewForces (Variables|Combat|GetDefenderPower))))
      (Default|CallOnTownDefenderPowerChanged _output_get))))

(event Custom|AddAlienForces
  (params (NewForces :type Float%20%28single-precision%29))
  (Math|Float|CompareFloat NewForces 0.0
    (:>
      (bind _output_get (Variables|Combat|SetAlienPower (+ NewForces (Variables|Combat|GetAlienPower))))
      (Default|CallOnTownAlienPowerChanged _output_get))))

(event Custom|TickCombat
  (params (DeltaTime :type Float%20%28single-precision%29))
  (bind _combatspeed (Variables|Combat|GetCombatSpeed))
  (bind _returnvalue (* DeltaTime _combatspeed))
  (Utilities|FlowControl|Sequence
    (:then_0
      (bind _output_get (Variables|Combat|SetAlienPower (Math|Float|Max(Float) (- (Variables|Combat|GetAlienPower) _returnvalue) 0.0)))
      (Default|CallOnTownAlienPowerChanged _output_get))
    (:then_1
      (bind _output_get_2 (Variables|Combat|SetDefenderPower (Math|Float|Max(Float) (- (Variables|Combat|GetDefenderPower) _returnvalue) 0.0)))
      (Default|CallOnTownDefenderPowerChanged _output_get_2))
    (:then_2
      (if (<= (Variables|Combat|GetDefenderPower) 0.0)
        (CallFunction|CaptureTown)))))

(event Custom|HandleTownRequestedHelp
  (params (TargetTown :type BP%20Base%20Town%20Object%20Reference) (IncomingForces :type Float%20%28single-precision%29))
  (if (Reinforcements|ShouldHelpTown TargetTown IncomingForces)
    (CallFunction|SendReinforcementstoTown TargetTown (Math|Float|Min(Float) (Reinforcements|GetDesiredReinforcementSize IncomingForces) (Reinforcements|GetMaxAvailableReinforcements)))))

(event Custom|SendReinforcementsToTown
  (params (TargetTown :type BP%20Base%20Town%20Object%20Reference) (ForcesToSend :type Float%20%28single-precision%29))
  (Utilities|IsValid TargetTown
    (:Is%20Valid
      (Utilities|FlowControl|Sequence
        (:then_0
          (bind _returnvalue (Game|SpawnActorfromClass (Variables|Reinforcements|GetReinforcementsClass) (Transformation|GetActorTransform) "AlwaysSpawn" 0 0))
          (Class|SpherePawn|SetPlanet _returnvalue (Variables|Default|GetMotherPlanet))
          (bind _returnvalue_2 (Class|SphericalCoordinateSystemBFL|To2D (Transformation|GetActorLocation)))
          (Class|SpherePawn|SetLocationonPlanet _returnvalue _returnvalue_2)
          (Class|SpherePawn|Moveto3D _returnvalue (Transformation|GetActorLocation TargetTown)))
        (:then_1
          (bind _output_get (Variables|Combat|SetDefenderPower (- (Variables|Combat|GetDefenderPower) ForcesToSend)))
          (Default|CallOnTownDefenderPowerChanged _output_get))))))

(event Custom|HandleTargetedByEnemies
  (params (IncomingForces :type Float%20%28single-precision%29))
  (Default|CallOnTownBeingTargetedDIspatcher self IncomingForces))

(event Custom|RotateWidgetToPlayerCamera
  (bind _widgetrootcomponent (Variables|Default|GetWidgetRootComponent))
  (Transformation|SetWorldRotation _widgetrootcomponent (Math|Rotator|FindLookatRotation (Transformation|GetWorldLocation _widgetrootcomponent) (Camera|GetCameraLocation (Game|GetPlayerCameraManager 0))) false false))

(event EventBeginPlay
  (bind _returnvalue (Actor|GetActorOfClass "/Game/Blueprints/BP_BasePlanet.BP_BasePlanet_C"))
  (Variables|Default|SetMotherPlanet _returnvalue)
  (Utilities|FlowControl|Sequence
    (:then_0
      (bind _returnvalue_2 (UserInterface|CreateWidget "/Game/HUD/Planet/WBP_TownBiomass.WBP_TownBiomass_C" 0 (Variables|Default|GetReward)))
      (UserInterface|SetWidget (Variables|Default|GetWidgetBiomassReward) _returnvalue_2))
    (:then_1
      (bind _returnvalue_3 (UserInterface|CreateWidget "/Game/HUD/Planet/WBP_TownAlienPower.WBP_TownAlienPower_C" 0 (Variables|Combat|GetAlienPower) self))
      (UserInterface|SetWidget (Variables|Default|GetWidgetAlienPower) _returnvalue_3))
    (:then_2
      (bind _returnvalue_4 (UserInterface|CreateWidget "/Game/HUD/Planet/WBP_TownDefenderPower.WBP_TownDefenderPower_C" 0 self (Variables|Combat|GetDefenderPower)))
      (UserInterface|SetWidget (Variables|Default|GetWidgetDefenderPower) _returnvalue_4))))

(event EventTick
  (params (DeltaSeconds :type Float%20%28single-precision%29))
  (Utilities|FlowControl|Sequence
    (:then_0
      (if (Combat|IsinCombat)
        (CallFunction|TickCombat DeltaSeconds)))
    (:then_1
      (CallFunction|RotateWidgettoPlayerCamera))))

(fn ConstructionScript
  (CallFunction|UpdateMesh)
  (CallFunction|SnaptothePlanet))

(fn IsTownCaptured
  (return (Variables|Combat|GetbIsCaptured)))

(fn IsinCombat
  (return (and (> (Variables|Combat|GetDefenderPower) 0.0) (> (Variables|Combat|GetAlienPower) 0.0))))

(fn CanEverSendReinforcements
  (return (Utilities|Enum|NotEqual(Enum) (Variables|Default|GetType) "NewEnumerator0")))

(fn CanSendReinforcementsNow
  (return (Math|Boolean|ANDBoolean (Reinforcements|CanEverSendReinforcements) (not (Combat|IsinCombat)) (not (Combat|IsTownCaptured)))))

(fn GetMaxAvailableReinforcements
  (return (select (Reinforcements|CanSendReinforcementsNow) 0.0 (/ (Variables|Combat|GetDefenderPower) 2.0))))

(fn ShouldHelpTown
  (params (TargetTown :type BP%20Base%20Town%20Object%20Reference) (IncomingForces :type Float%20%28single-precision%29))
  (Utilities|IsValid TargetTown
    (:Is%20Valid
      (if (Reinforcements|CanSendReinforcementsNow)
        (if (not (Combat|IsTownCaptured TargetTown))
          (return (< IncomingForces (Math|Float|Min(Float) (Reinforcements|GetDesiredReinforcementSize IncomingForces) (Reinforcements|GetMaxAvailableReinforcements))))
          (else
            _))))
    (:Is%20Not%20Valid
      _))
  (return false))

(fn GetDesiredReinforcementSize
  (params (EnemyForces :type Float%20%28single-precision%29))
  (return (* EnemyForces (Variables|Reinforcements|GetMinOverwhelmCoefficient))))

(fn GetReinforcementsSpawnTransform
  (params (DestinationTown :type BP%20Base%20Town%20Object%20Reference))
  (return (Transformation|GetActorTransform)))