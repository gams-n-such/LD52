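; Game mode Blueprint that decides when the game is won or lost from the player's biomass, power and captured city count.
; On BeginPlay it binds to change events on the first player's BP_PlayerState, setting flags for empty resources and full city capture.
; Capturing the maximum number of cities calls GameWin; both resources reaching zero before that calls GameOver.
; GameWin and GameOver are empty stubs here.
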(event Custom|EventOnChangeCurrentBiomass
  (params (CurrentBiomass :type Float%20%28single-precision%29))
  (bind _output_get (Variables|Default|SetIsBiomassEmpty (Math|Float|NearlyEqual(Float) CurrentBiomass 0.0 1e-06)))
  (if _output_get
    (CallFunction|CheckGameOver)))

(event Custom|EventOnChangeCurrentPower
  (params (CurrentPower :type Float%20%28single-precision%29))
  (bind _output_get (Variables|Default|SetIsPowerEmpty (Math|Float|NearlyEqual(Float) CurrentPower 0.0 1e-06)))
  (if _output_get
    (CallFunction|CheckGameOver)))

(event Custom|CheckGameOver
  (if (Math|Boolean|ANDBoolean (Variables|Default|GetIsBiomassEmpty) (Variables|Default|GetIsPowerEmpty) (not (Variables|Default|Get%20IsAllCitiesBeenCaptured)))
    (CallFunction|GameOver)))

(event Custom|GameOver)

(event Custom|EventOnChangeCapturedSitiesCount
  (params (CurrentCapturedСities :type Integer))
  (bind _output_get (Variables|Default|Set%20IsAllCitiesBeenCaptured (== CurrentCapturedСities (Variables|Default|GetMaxCapturedСities))))
  (if _output_get
    (CallFunction|GameWin)))

(event Custom|GameWin)

(event EventBeginPlay
  (bind _asbp_player_state (Utilities|Casting|CastToBP_PlayerState (Variables|/Script/Engine.Controller|GetPlayerState (Game|GetPlayerController 0))))
  (EventDispatchers|BindEventtoOnChangeCurrentBiomass _asbp_player_state (EventDispatchers|CreateEvent :!event Custom|EventOnChangeCurrentBiomass))
  (EventDispatchers|BindEventtoOnChangeCurrentPower _asbp_player_state (EventDispatchers|CreateEvent :!event Custom|EventOnChangeCurrentPower))
  (EventDispatchers|BindEventtoOnChangeCapturedCitiesCount _asbp_player_state (EventDispatchers|CreateEvent :!event Custom|EventOnChangeCapturedSitiesCount)))

(fn ConstructionScript)