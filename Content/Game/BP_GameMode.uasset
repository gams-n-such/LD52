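; Game mode that decides when a planet is won or lost and shows the end-of-planet screen.
; On BeginPlay it counts all BP_BaseTown actors and binds to the player state's biomass, power and captured-city change events.
; Capturing every town triggers a win; near-zero power with no affordable skill, checked on biomass or power changes, triggers a loss.
; Both outcomes open WBP_EndPlanet with a win flag.
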(event Custom|EventOnChangeCurrentBiomass
  (params (CurrentBiomass :type Float%20%28single-precision%29))
  (CallFunction|CheckLose))

(event Custom|EventOnChangeCurrentPower
  (params (CurrentPower :type Float%20%28single-precision%29))
  (Variables|Default|SetIsPowerEmpty (Math|Float|NearlyEqual(Float) CurrentPower 0.0 1e-06))
  (CallFunction|CheckLose))

(event Custom|CheckLose
  (bind _newparam (Default|CheckCanAffordAnySkill (Variables|Default|GetAs%20BP%20Player%20State)))
  (if (and (Variables|Default|GetIsPowerEmpty) (not _newparam))
    (CallFunction|GameLose)))

(event Custom|GameLose
  (bind _returnvalue (UserInterface|CreateWidget "/Game/HUD/WBP_EndPlanet.WBP_EndPlanet_C"))
  (UserInterface|Viewport|AddtoViewport _returnvalue 0))

(event Custom|EventOnChangeCapturedSitiesCount
  (params (CurrentCapturedСities :type Integer))
  (if (== CurrentCapturedСities (Variables|Default|GetMaxCapturedСities))
    (CallFunction|GameWin)))

(event Custom|GameWin
  (bind _returnvalue (UserInterface|CreateWidget "/Game/HUD/WBP_EndPlanet.WBP_EndPlanet_C" 0 true))
  (UserInterface|Viewport|AddtoViewport _returnvalue 0))

(event EventBeginPlay
  (Utilities|FlowControl|Sequence
    (:then_0
      (bind _outactors (Actor|GetAllActorsOfClass "/Game/Blueprints/BP_BaseTown.BP_BaseTown_C"))
      (Variables|Default|SetMaxCapturedСities (Utilities|Array|Length _outactors)))
    (:then_1
      (bind _asbp_player_state (Utilities|Casting|CastToBP_PlayerState (Variables|/Script/Engine.Controller|GetPlayerState (Game|GetPlayerController 0))))
      (bind _output_get (Variables|Default|SetAs%20BP%20Player%20State _asbp_player_state))
      (EventDispatchers|BindEventtoOnChangeCurrentBiomass _output_get (EventDispatchers|CreateEvent :!event Custom|EventOnChangeCurrentBiomass))
      (EventDispatchers|BindEventtoOnChangeCurrentPower _output_get (EventDispatchers|CreateEvent :!event Custom|EventOnChangeCurrentPower))
      (EventDispatchers|BindEventtoOnChangeCapturedCitiesCount _output_get (EventDispatchers|CreateEvent :!event Custom|EventOnChangeCapturedSitiesCount)))))

(fn ConstructionScript)

(fn NewFunction0)